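; Player controller for a Pokémon-style game that restores the saved character on BeginPlay, or calls SelectWb on the game instance when no save exists.
; Save writes the game instance's chosen sex and stored position, plus the player character's class, to a single slot.
; Load copies sex back, spawns that class at the saved position with zero rotation, possesses it and sets game-only input, or calls Save if the slot is empty.
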(event `self.ReceiveBeginPlay`
  (bind _returnvalue (`GameplayStatics.DoesSaveGameExist` "slot"))
  (if _returnvalue
    (`self.load`)
    (else
      (bind _aspokegameinstance (cast `/Game/blueprints/save_game/pokegameinstance` (`GameplayStatics.GetGameInstance`)))
      (`/Game/blueprints/save_game/pokegameinstance.select wb` _aspokegameinstance))))

(fn `load`
  (bind _returnvalue (`GameplayStatics.GetPlayerController` 0))
  (bind _returnvalue_2 (`GameplayStatics.DoesSaveGameExist` "slot"))
  (if _returnvalue_2
    (bind _returnvalue_3 (`GameplayStatics.LoadGameFromSlot` "slot"))
    (bind _assexselectionsave (cast `/Game/blueprints/save_game/sexselectionsave` _returnvalue_3))
    (bind _aspokegameinstance (cast `/Game/blueprints/save_game/pokegameinstance` (`GameplayStatics.GetGameInstance`)))
    (set `/Game/blueprints/save_game/pokegameinstance.sexchosen` (`/Game/blueprints/save_game/sexselectionsave.sex` _assexselectionsave) _aspokegameinstance)
    (bind _returnvalue_4 (`|SpawnActorFromClass` (`/Game/blueprints/save_game/sexselectionsave.actor` _assexselectionsave) (`KismetMathLibrary.MakeTransform` (`/Game/blueprints/save_game/sexselectionsave.transform` _assexselectionsave)) "AlwaysSpawn" "OverrideRootScale" null null))
    (`self.Possess` _returnvalue _returnvalue_4)
    (`WidgetBlueprintLibrary.SetInputMode_GameOnly` _returnvalue)
    (set `PlayerController.bShowMouseCursor` false _returnvalue)
    (else
      (`self.save`))))

(fn `save`
  (bind _returnvalue (`GameplayStatics.CreateSaveGameObject` "/Game/blueprints/save_game/sexselectionsave.sexselectionsave_C"))
  (bind _assexselectionsave (cast `/Game/blueprints/save_game/sexselectionsave` _returnvalue))
  (bind _aspokegameinstance (cast `/Game/blueprints/save_game/pokegameinstance` (`GameplayStatics.GetGameInstance`)))
  (set `/Game/blueprints/save_game/sexselectionsave.sex` (`/Game/blueprints/save_game/pokegameinstance.sexchosen` _aspokegameinstance) _assexselectionsave)
  (set `/Game/blueprints/save_game/sexselectionsave.transform` (`/Game/blueprints/save_game/pokegameinstance.actor transform` _aspokegameinstance) _assexselectionsave)
  (set `/Game/blueprints/save_game/sexselectionsave.actor` (`GameplayStatics.GetObjectClass` (`GameplayStatics.GetPlayerCharacter` 0)) _assexselectionsave)
  (`GameplayStatics.SaveGameToSlot` _assexselectionsave "slot"))

(fn `UserConstructionScript`)