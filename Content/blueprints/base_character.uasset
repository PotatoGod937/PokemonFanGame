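; Base player character with axis movement, yaw look, hold-to-sprint and a random battle encounter counter for long grass.
; LookForBattle seeds a random countdown when overlapping an in_long_grass actor, though nothing here calls it.
; The counter subtracts random amounts and uses the RandomTimer timeline to lerp toward the reduced value, re-running itself until zero triggers EnterBattle.
; EnterBattle is an empty stub.
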(event `InputAxis|MoveForward`
  (params (AxisValue :type "Float (single-precision)"))
  (bind _returnvalue (`GameplayStatics.GetPlayerCharacter` 0))
  (bind _output_get (set `self.moveforward_value` AxisValue))
  (`self.AddMovementInput` _returnvalue (`self.GetActorForwardVector` _returnvalue) _output_get false))

(event `InputAxis|MoveRight`
  (params (AxisValue :type "Float (single-precision)"))
  (bind _returnvalue (`GameplayStatics.GetPlayerCharacter` 0))
  (bind _output_get (set `self.Move left Value` AxisValue))
  (`self.AddMovementInput` _returnvalue (`self.GetActorRightVector` _returnvalue) _output_get false))

(event `InputAxis|look`
  (params (AxisValue :type "Float (single-precision)"))
  (`self.AddControllerYawInput` AxisValue))

(event `InputAction|Sprint`
  (params (Key :type "Key Structure"))
  (bind _charactermovement (`self.CharacterMovement`))
  (:`Pressed`
    (set `CharacterMovementComponent.MaxWalkSpeed` 900.0 _charactermovement))
  (:`Released`
    (set `CharacterMovementComponent.MaxWalkSpeed` 600.0 _charactermovement)))

(event `random encounter counter`
  ;[1 1 1] random encounter counter
  (if (`self.stop counting`)
    (bind (_direction _time) (`Timeline|random timer` :!via `Stop` :!label _label)
      (:`Update`
        (if (<= (`KismetMathLibrary.Lerp` (`self.count for battle`) (stale _count) _time) 0.0)
          (`self.enter battle`)
          (else
            (`self.random encounter counter`)))))
    (else
      (bind _count (`self.random encounter time`))
      (goto _label))))

(fn `enter battle`)

(fn `look for battle`
  (for _array_element (`self.GetOverlappingActors` null)
    (bind _asin_long_grass (cast `/Game/blueprints/long_grass_battle/in_long_grass` _array_element))
    (if (`self.IsOverlappingActor` _asin_long_grass)
      (set `self.stop counting` false)
      (set `self.count for battle` (`KismetMathLibrary.RandomFloatInRange` 35.0 85.0))
      (`self.random encounter counter`))))

(fn `random encounter time`
  (returns (count :type "Float (double-precision)"))
  (bind _returnvalue (- (`self.count for battle`) (`KismetMathLibrary.RandomFloatInRange` (`self.random battle counter min`) (`self.random battle counter max`))))
  (set `self.count for battle` _returnvalue)
  (return _returnvalue))

(fn `UserConstructionScript`)