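; Pikachu Pokémon actor that follows the player by AI movement.
; Its moverilou event casts the player character to base_character, issues an AI MoveTo toward it, then re-calls itself after a short delay to keep refreshing the chase.
; Tick starts that loop through a longer Delay instead of BeginPlay, which is empty, and keeps re-calling it each time the delay completes.
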(event `self.ReceiveBeginPlay`)

(event `moverilou`
  (bind _asbase_character (cast `/Game/blueprints/base_character` (`GameplayStatics.GetPlayerCharacter` 0)))
  (`|AIMoveTo` self (0.0 0.0 0.0) _asbase_character
    (:`then`
      _)
    (:`OnSuccess`
      _)
    (:`OnFail`
      _))
  (`KismetSystemLibrary.Delay` 0.2)
  (`self.moverilou`))

(event `self.ReceiveTick`
  (params (DeltaSeconds :type "Float (single-precision)"))
  (`KismetSystemLibrary.Delay` 2.0)
  (`self.moverilou`))

(fn `UserConstructionScript`
  (`parent.UserConstructionScript`))