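; Riolu Pokémon actor that follows the player character around the world.
; Tick checks the player's Isinbattle flag and, while it is false, calls moverilou after a 2-second Delay.
; moverilou sends an AI move to the player's Sphere component location and re-calls itself every 0.2 seconds.
; That loop does not recheck the battle flag, so it keeps running once started.
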(event `self.ReceiveBeginPlay`)

(event `moverilou`
  (bind _asbase_character (cast `/Game/blueprints/base_character` (`GameplayStatics.GetPlayerCharacter` 0)))
  (`|AIMoveTo` self (`SceneComponent.K2_GetComponentLocation` (`/Game/blueprints/base_character.Sphere` _asbase_character)) null
    (:`then`
      _)
    (:`OnSuccess`
      _)
    (:`OnFail`
      _))
  (`KismetSystemLibrary.Delay` 0.2)
  (`self.moverilou`))

(event `self.ReceiveTick`
  (params (DeltaSeconds :type "Float (single-precision)"))
  (bind _asbase_character (cast `/Game/blueprints/base_character` (`GameplayStatics.GetPlayerCharacter` 0)))
  (if (not (`/Game/blueprints/base_character.isinbattle` _asbase_character))
    (`KismetSystemLibrary.Delay` 2.0)
    (`self.moverilou`)))

(fn `UserConstructionScript`
  (`parent.UserConstructionScript`))